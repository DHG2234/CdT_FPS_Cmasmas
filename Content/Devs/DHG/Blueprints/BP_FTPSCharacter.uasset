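; BP_FTPSCharacter is a character Blueprint with first-person and third-person camera components and a melee detector.
; At BeginPlay and on each F press, which flips UseFirstPersonView, ChangeCamera sets camera active states.
; Both cameras receive the same un-inverted flag, with the TPS camera wired in twice, so they activate and deactivate together.
; Melee detector overlaps only print the other actor's name.
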(event OnComponentBeginOverlap(MeleeDetectorComponent)
  (params (OverlappedComponent :type Primitive%20Component%20Object%20Reference) (OtherActor :type Actor%20Object%20Reference) (OtherComp :type Primitive%20Component%20Object%20Reference) (OtherBodyIndex :type Integer) (bFromSweep :type Boolean) (SweepResult :type Hit%20Result%20Structure%20%28by%20ref%29))
  (Development|PrintString (Utilities|GetDisplayName OtherActor)))

(event Custom|ChangeCamera
  (Components|Activation|SetActive (Variables|Default|GetFPSCameraComponent) (Variables|Default|GetbUseFirstPersonView) false)
  (Components|Activation|SetActive (Variables|Default|GetTPSCameraComponent) (Variables|Default|GetbUseFirstPersonView) false))

(event EventBeginPlay
  (CallFunction|ChangeCamera))

(event Collision|EventActorBeginOverlap
  (params (OtherActor :type Actor%20Object%20Reference)))

(event EventTick
  (params (DeltaSeconds :type Float%20%28single-precision%29)))

(event Input|KeyboardEvents|F
  (params (Key :type Key%20Structure :default "None"))
  (:Pressed
    (Variables|Default|SetbUseFirstPersonView (not (Variables|Default|GetbUseFirstPersonView)))
    (CallFunction|ChangeCamera)))

(fn ConstructionScript)